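; Actor component that simulates arrow flight, launching its owner along its forward vector at a set speed.
; Each tick it line-traces the next step on Visibility with debug drawing, otherwise moves the owner, applies exaggerated downward gravity and rotates it along the path.
; A hit snaps the owner to the impact point and cancels the timer that would destroy it after a fixed lifetime; ticking is not stopped.
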(event `Target Hit`
  (params (`Hit Location` :type "Vector Structure") (`Hit Actor` :type "Actor Object Reference"))
  (`|ExecutionSequence`
    (:`then_0`
      (`KismetSystemLibrary.K2_ClearAndInvalidateTimerHandle` (`self.DestroyEvent`)))
    (:`then_1`
      (`Actor.K2_SetActorLocation` (`self.GetOwner`) `Hit Location` false false))))

(event `self.ReceiveBeginPlay`
  (set `self.Velocity` (* (`Actor.GetActorForwardVector` (`self.GetOwner`)) (`self.Speed`)))
  (set `self.StartPos` (`Actor.K2_GetActorLocation` (`self.GetOwner`)))
  (bind _returnvalue (`KismetSystemLibrary.K2_SetTimerDelegate` (delegate `Destroy Arrow`) 20.0))
  (set `self.DestroyEvent` _returnvalue))

(event `Destroy Arrow`
  (`Actor.K2_DestroyActor` (`self.GetOwner`)))

(event `self.ReceiveTick`
  (params (DeltaSeconds :type "Float (single-precision)"))
  (set `self.Delta Time` DeltaSeconds)
  (set `self.StartPos` (`Actor.K2_GetActorLocation` (`self.GetOwner`)))
  (set `self.EndPos` (+ (`self.StartPos`) (* (`self.Velocity`) (`self.Delta Time`))))
  (bind (_outhit _returnvalue) (`KismetSystemLibrary.LineTraceSingle` :`Start` (`self.StartPos`) :`End` (`self.EndPos`) :`TraceChannel` "TraceTypeQuery1" :`DrawDebugType` "ForDuration" :`DrawTime` 6.0))
  (if _returnvalue
    (`self.Target Hit` (`.ImpactPoint` (`GameplayStatics.BreakHitResult` _outhit)) (`.HitActor` (`GameplayStatics.BreakHitResult` _outhit)))
    (else
      (`Actor.K2_SetActorLocation` (`self.GetOwner`) (`self.EndPos`) false false)
      (set `self.Velocity` (- (`self.Velocity`) (* (`KismetMathLibrary.MakeVector` 0.0 0.0 (* 980.0 10.0)) (`self.Delta Time`))))
      (`Actor.K2_SetActorRotation` (`self.GetOwner`) (`KismetMathLibrary.FindLookAtRotation` (`self.StartPos`) (`self.EndPos`)) false))))