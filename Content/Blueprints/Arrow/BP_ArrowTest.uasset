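; BP_ArrowTest is a test arrow projectile that moves along an analytic parabola from start position, direction, speed and gravity.
; Tick sets the actor's location on the curve, keeping its rotation.
; Async physics tick, gated on initialization and negative Time, line-traces between predicted points and destroys the arrow on a hit.
; The trace passes the difference vector (end minus start) as its End location, rather than the next point.
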(event `self.ReceiveAsyncPhysicsTick`
  (params (DeltaSeconds :type "Float (single-precision)") (SimSeconds :type "Float (single-precision)"))
  (if (`self.isInitalized`)
    (if (< (`self.time`) 0.0)
      (set `self.time` (- (`self.time`) DeltaSeconds))
      (set `self.nextTime` (+ (`self.currentTime`) SimSeconds))
      (bind _endpoint (`self.FindPointOnParabola` (`self.currentTime`)))
      (set `self.currentPoint` _endpoint)
      (bind _endpoint_2 (`self.FindPointOnParabola` (`self.nextTime`)))
      (set `self.nextPoint` _endpoint_2)
      (bind _hit (`self.Cast ray Between POints` (`self.currentPoint`) (`self.nextPoint`)))
      (if _hit
        (`self.K2_DestroyActor`)))))

(event `self.ReceiveTick`
  (params (DeltaSeconds :type "Float (single-precision)"))
  (bind (_returnvalue_location _returnvalue_rotation _returnvalue_scale) (`KismetMathLibrary.BreakTransform` (`self.GetTransform`)))
  (if (and (`self.isInitalized`) (< (`self.time`) 0.0))
    _
    (else
      _))
  (set `self.currentTime` (- DeltaSeconds (`self.time`)))
  (bind _endpoint (`self.FindPointOnParabola` (`self.currentTime`)))
  (bind _output_get (set `self.currentPoint` _endpoint))
  (`self.K2_SetActorTransform` (`KismetMathLibrary.MakeTransform` _output_get _returnvalue_rotation _returnvalue_scale)))

(fn `Cast ray Between POints`
  (params (Startpoint :type "Vector Structure") (Endpoint :type "Vector Structure"))
  (returns (Hit :type Boolean) (RaycastHit1 :type "HitResult Structure"))
  (bind (_outhit _returnvalue) (`KismetSystemLibrary.LineTraceSingle` Startpoint (- Endpoint Startpoint) "TraceTypeQuery1"))
  (return _returnvalue _outhit))

(fn `FindPointOnParabola`
  (params (Time :type "Float (double-precision)"))
  (returns (EndPoint :type "Vector Structure"))
  (locals (Point :type "Vector Structure") (GravityVec :type "Vector Structure"))
  (set `local.Point` (+ (`self.startPos`) (* (`self.startForward`) (`self.speed`) (`self.time`))))
  (set `local.GravityVec` (* (`KismetMathLibrary.Vector_Down`) (`self.gravity`) (`self.time`) (`self.time`)))
  (return (+ (`local.Point`) (`local.GravityVec`))))

(fn `UserConstructionScript`
  (set `self.isInitalized` true))