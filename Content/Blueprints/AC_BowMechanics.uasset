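; Bow component that handles draw strength and arrow firing for the player character.
; NotchBow uses a Gate and short Delay to throttle draw increments up to MaxDrawStrength, printing the value as debug output.
; FireBow spawns BP_ArrowBallistics at the arrow spawn point along the camera rotation, scaling speed by DrawStrength, then notifies the character.
; NotchDown lowers the draw in larger steps than NotchUp raises it; ReloadBow is an empty stub.
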(event `Notch Bow`
  (`/Engine/EditorBlueprintResources/StandardMacros.Gate` false :!label _label
    (:`Exit`
      (`self.NotchUp`)
      (`|ExecutionSequence`
        (:`then_0`
          (goto _label :!via `Close`))
        (:`then_1`
          (`KismetSystemLibrary.Delay` 0.1)
          (`KismetSystemLibrary.PrintString` (`KismetStringLibrary.Conv_DoubleToString` (`self.drawStrength`)))
          (goto _label :!via `Open`))))))

(event `Reset Bow`
  (`/Game/ThirdPerson/Blueprints/BP_ThirdPersonCharacter.Bow Fired` (`self.playerCharater`)))

(fn `FireBow`
  (bind _playercharater (`self.playerCharater`))
  (`|SpawnActorFromClass` "/Game/Blueprints/Arrow/BP_ArrowBallistics.BP_ArrowBallistics_C" (`KismetMathLibrary.MakeTransform` (`SceneComponent.K2_GetComponentLocation` (`/Game/ThirdPerson/Blueprints/BP_ThirdPersonCharacter.Arrow Spawn Point` _playercharater)) (`SceneComponent.K2_GetComponentRotation` (`/Game/ThirdPerson/Blueprints/BP_ThirdPersonCharacter.FollowCamera` _playercharater))) "Undefined" "MultiplyWithRoot" null (`self.drawStrength`) null)
  (`self.Reset Bow`))

(fn `NotchDown`
  (bind _drawstrength (`self.drawStrength`))
  (if (<= _drawstrength 0.0)
    (`self.UndrawBow`)
    (else
      (`/Engine/EditorBlueprintResources/StandardMacros.DecrementFloat` _drawstrength))))

(fn `NotchUp`
  (bind _drawstrength (`self.drawStrength`))
  (if (not (>= _drawstrength (`self.maxDrawStrength`)))
    (set `self.drawStrength` (+ _drawstrength 0.1))))

(fn `ReloadBow`)

(fn `UndrawBow`
  (set `self.drawStrength` 0.0))